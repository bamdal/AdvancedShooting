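; BP_JMSShootingChar is a shooter character that switches between unarmed, pistol and rifle stances and between walking and jogging gates.
; The weapon-switch input sets EquipGun and links the matching animation layer class on the mesh.
; Holding aim switches to the Walking gate and releasing it returns to Jogging.
; UpdateGate notifies the AnimInstance and applies that gate's speed, acceleration and braking settings from the GateSettings map to CharacterMovement.
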(event Input|EnhancedActionEvents|EnhancedInputActionIA_AdvancedShooting_SwichWeapon
  (params (ActionValue :type Float%20%28double-precision%29) (ElapsedSeconds :type Float%20%28double-precision%29) (TriggeredSeconds :type Float%20%28double-precision%29) (InputAction :type Input%20Action%20Object%20Reference :default "/Game/Characters/Input/IA/IA_AdvancedShooting_SwichWeapon.IA_AdvancedShooting_SwichWeapon"))
  (bind _mesh (Variables|Character|GetMesh))
  (switch int (Math|Float|Truncate ActionValue)
    (:Default
      (Development|PrintString "BP_JMSShootingChar EquipGun Null"))
    (:1
      (Variables|Default|SetEquipGun "UnArmed")
      (Components|SkeletalMesh|AnimationBlueprintLinking|LinkAnimClassLayers _mesh "/Game/ALS/ABP/ABP_Layers_UnArmed.ABP_Layers_UnArmed_C"))
    (:2
      (Variables|Default|SetEquipGun "Pistol")
      (Components|SkeletalMesh|AnimationBlueprintLinking|LinkAnimClassLayers _mesh "/Game/ALS/ABP/ABP_Layers_Pistol.ABP_Layers_Pistol_C"))
    (:3
      (Variables|Default|SetEquipGun "Rifle")
      (Components|SkeletalMesh|AnimationBlueprintLinking|LinkAnimClassLayers _mesh "/Game/ALS/ABP/ABP_Layers_Rifle.ABP_Layers_Rifle_C"))))

(event Input|EnhancedActionEvents|EnhancedInputActionIA_AdvancedShooting_AIM
  (params (ActionValue :type Boolean) (ElapsedSeconds :type Float%20%28double-precision%29) (TriggeredSeconds :type Float%20%28double-precision%29) (InputAction :type Input%20Action%20Object%20Reference :default "/Game/Characters/Input/IA/IA_AdvancedShooting_AIM.IA_AdvancedShooting_AIM"))
  (:Started
    (CallFunction|UpdateGate "Walking"))
  (:Completed
    (CallFunction|UpdateGate "Jogging")))

(event EventBeginPlay
  (Components|SkeletalMesh|AnimationBlueprintLinking|LinkAnimClassLayers (Variables|Character|GetMesh) "/Game/ALS/ABP/ABP_Layers.ABP_Layers_C")
  (CallFunction|UpdateGate (Variables|Default|GetCurrentGate)))

(event Collision|EventActorBeginOverlap
  (params (OtherActor :type Actor%20Object%20Reference)))

(event EventTick
  (params (DeltaSeconds :type Float%20%28single-precision%29)))

(fn ConstructionScript)

(fn UpdateGate
  (params (Gate :type E_Gate%20Enum :default "Walking"))
  (bind _charactermovement (Variables|Character|GetCharacterMovement))
  (bind _output_get (Variables|Default|SetCurrentGate Gate))
  (Class|BPIABPas|ReceiveCurrentGate(Message) (Components|SkeletalMesh|GetAnimInstance (Variables|Character|GetMesh)) _output_get)
  (Utilities|FlowControl|Sequence
    (:then_0
      (Variables|/Script/Engine.CharacterMovementComponent|SetMaxWalkSpeed _charactermovement (.MaxWalkSpeed (Utilities|Struct|BreakS_GateSetting (.Value (Utilities|Map|Find (Variables|Default|GetGateSettings) _output_get)))))
      (Variables|/Script/Engine.CharacterMovementComponent|SetMaxAcceleration _charactermovement (.MaxAcceleration (Utilities|Struct|BreakS_GateSetting (.Value (Utilities|Map|Find (Variables|Default|GetGateSettings) _output_get)))))
      (Variables|/Script/Engine.CharacterMovementComponent|SetBrakingDecelerationWalking _charactermovement (.BrakingDeceleration (Utilities|Struct|BreakS_GateSetting (.Value (Utilities|Map|Find (Variables|Default|GetGateSettings) _output_get)))))
      (Variables|/Script/Engine.CharacterMovementComponent|SetBrakingFrictionFactor _charactermovement (.BrakingFrictionFactor (Utilities|Struct|BreakS_GateSetting (.Value (Utilities|Map|Find (Variables|Default|GetGateSettings) _output_get)))))
      (Variables|/Script/Engine.CharacterMovementComponent|SetBrakingFriction _charactermovement (.BrakingFiction (Utilities|Struct|BreakS_GateSetting (.Value (Utilities|Map|Find (Variables|Default|GetGateSettings) _output_get)))))
      (Variables|/Script/Engine.CharacterMovementComponent|SetbUseSeparateBrakingFriction _charactermovement (.UseSeparateBrakingFiction (Utilities|Struct|BreakS_GateSetting (.Value (Utilities|Map|Find (Variables|Default|GetGateSettings) _output_get))))))))