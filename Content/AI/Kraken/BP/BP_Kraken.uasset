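; Kraken enemy character that fights the player, feeding its behavior tree through blackboard keys for the target player and death.
; Damage varies by hit bone (weak shell, vulnerable beak), updates a health bar and spawns Niagara damage numbers.
; A detection sphere sets the target and toggles the bar; non-lethal hits also set the target.
; Random attack montages enable mesh-overlap damage and knockback, capped at three hits per attack.
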(event OnComponentBeginOverlap(Sphere)
  (params (OverlappedComponent :type Primitive%20Component%20Object%20Reference) (OtherActor :type Actor%20Object%20Reference) (OtherComp :type Primitive%20Component%20Object%20Reference) (OtherBodyIndex :type Integer) (bFromSweep :type Boolean) (SweepResult :type Hit%20Result%20Structure%20%28by%20ref%29))
  (bind _returnvalue (AI|GetBlackboard 0))
  ;[0.15 0.15 0.15 0.5] 감지범위내에 플레이어 발견
  (bind _asbp_jmsshooting_char (Utilities|Casting|CastToBP_JMSShootingChar OtherActor))
  (Utilities|IsValid _returnvalue
    (:Is%20Valid
      (AI|Components|Blackboard|SetValueasObject _returnvalue (Utilities|Name|MakeLiteralName "Player") _asbp_jmsshooting_char)
      (Widget|SetVisibility (Variables|Default|GetHealthbar) "Visible"))))

(event OnComponentEndOverlap(Sphere)
  (params (OverlappedComponent :type Primitive%20Component%20Object%20Reference) (OtherActor :type Actor%20Object%20Reference) (OtherComp :type Primitive%20Component%20Object%20Reference) (OtherBodyIndex :type Integer))
  (Utilities|Casting|CastToBP_JMSShootingChar OtherActor)
  (Widget|SetVisibility (Variables|Default|GetHealthbar) "Collapsed"))

(event OnComponentBeginOverlap(Mesh)
  (params (OverlappedComponent :type Primitive%20Component%20Object%20Reference) (OtherActor :type Actor%20Object%20Reference) (OtherComp :type Primitive%20Component%20Object%20Reference) (OtherBodyIndex :type Integer) (bFromSweep :type Boolean) (SweepResult :type Hit%20Result%20Structure%20%28by%20ref%29))
  (bind _damageamount (Variables|Default|GetDamageAmount))
  (bind _asbp_jmsshooting_char (Utilities|Casting|CastToBP_JMSShootingChar OtherActor))
  (if (and (Variables|Default|GetIsAttacking) (<= (Variables|Default|GetDamageAmount) 2))
    (Class|JMSShootingChar|DecreaseHealth _asbp_jmsshooting_char (Math|Random|RandomFloatinRange 5.0 1e+01))
    (Math|Integer|IncrementInt _damageamount
      (:%20%20
        (Development|PrintString (Utilities|String|ToString(Integer) _damageamount))
        (Character|LaunchCharacter _asbp_jmsshooting_char (* (Math|Vector|Normalize (- (Transformation|GetWorldLocation (Variables|/Script/Engine.Character|GetMesh _asbp_jmsshooting_char)) (Transformation|GetWorldLocation (Variables|Character|GetMesh)))) 1e+03) true false)))))

(event EventBeginPlay
  (Variables|Default|SetOldHealth (Variables|Default|GetOldMaxHealth))
  ;[0.15 0.15 0.15 0.5] Healthbar 생성
  (bind _returnvalue (UserInterface|CreateWidget "/Game/AI/Kraken/BP/WBP_KrakenHealth.WBP_KrakenHealth_C"))
  (bind _output_get (Variables|Default|SetHealthbar _returnvalue))
  (UserInterface|Viewport|AddtoViewport _output_get 0)
  (CallFunction|UpdateHealth)
  (Widget|SetVisibility (Variables|Default|GetHealthbar) "Collapsed"))

(event EventDamage
  (params (HitBoneName :type Name :default "None") (ImpactLocation :type Vector :default "0, 0, 0"))
  (bind _returnvalue (AI|GetBlackboard 0))
  (Variables|Default|SetImpact%20Location ImpactLocation)
  (if (not (Variables|Default|GetIsDead))
    ;[0.15 0.15 0.15 0.5] 피격 위치에 맞는데미지
    (switch name HitBoneName
      (:Default
        (Variables|Default|SetOldDamageRecieved (Math|Random|RandomFloatinRange 25.0 5e+01)))
      (:KRAKEN_SHELL
        (Variables|Default|SetOldDamageRecieved (Math|Random|RandomFloatinRange 3.0 1e+01)))
      (:KRAKEN_BEAK_LEFT
        (Variables|Default|SetOldDamageRecieved (Math|Random|RandomFloatinRange 5e+01 1e+02) :!label _label))
      (:KRAKEN_BEAK_LOWER
        (goto _label))
      (:KRAKEN_BEAK_RIGHT
        (goto _label))
      (:KRAKEN_BEAK_UPPER
        (goto _label)))
    (bind _output_get (Variables|Default|SetOldHealth (- (Variables|Default|GetOldHealth) (Variables|Default|GetOldDamageRecieved))))
    (CallFunction|UpdateHealth)
    ;[0.15 0.15 0.15 0.5] HitNumber Niagara
    (bind _returnvalue_2 (Niagara|SpawnSystematLocation "/Game/Effects/Particles/Impacts/NS_DamageNumbers.NS_DamageNumbers" "0, 0, 0"))
    (Class|NiagaraDataInterfaceArrayFunctionLibrary|SetNiagaraArrayVector4 _returnvalue_2 "User.DamageInfo" (Utilities|Array|MakeArray (Math|Vector4|MakeVector4 (.x (Variables|Default|GetImpact%20Location)) (.y (Variables|Default|GetImpact%20Location)) (.z (Variables|Default|GetImpact%20Location)) (Variables|Default|GetOldDamageRecieved))))
    (if (< _output_get 0.0)
      ;[0.15 0.15 0.15 0.5] Die
      (Variables|Default|SetIsDead true)
      (Animation|Montage|PlayMontage (Variables|Character|GetMesh) "/Game/AI/Kraken/Animations/AM_KRAKEN_death.AM_KRAKEN_death"
        (:then
          (AI|Components|Blackboard|SetValueasBool (AI|GetBlackboard 0) (Utilities|Name|MakeLiteralName "IsDeadKey") (Variables|Default|GetIsDead))))
      (else
        ;[0.15 0.15 0.15 0.5] Hit 시 플레이어 추격
        (bind _asbp_jmsshooting_char (Utilities|Casting|CastToBP_JMSShootingChar (Game|GetPlayerCharacter 0)))
        (Utilities|IsValid _returnvalue
          (:Is%20Valid
            (AI|Components|Blackboard|SetValueasObject _returnvalue (Utilities|Name|MakeLiteralName "Player") _asbp_jmsshooting_char)))))))

(event EventAttack
  (Variables|Default|SetIsAttacking true)
  (Animation|Montage|PlayMontage (Variables|Character|GetMesh) (.OutItem (Utilities|Array|Random (Variables|Default|GetAttackMontage)))
    (:OnCompleted
      (Variables|Default|SetIsAttacking false)
      (Variables|Default|SetDamageAmount 0))))

(fn ConstructionScript)

(fn UpdateHealth
  (Variables|/Game/AI/Kraken/BP/WBP_KrakenHealth.WBP_KrakenHealth_C|SetHealthPercent (Variables|Default|GetHealthbar) (/ (Variables|Default|GetOldHealth) (Variables|Default|GetOldMaxHealth))))